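; Base weapon Blueprint that gives its owning Character data-driven attack actions and skills, with empty hooks for equip, action and sub-action logic.
; On BeginPlay it caches ActionTable rows and the owner, then getters filter rows by WeaponType and Skill flag for per-index properties.
; PlayAction plays the montage and signals move or stop via IWeapon, always checking the non-skill CanMove.
; SendDamage excludes self and owner, crediting player controller 0.
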(event EventBeginPlay
  (Utilities|FlowControl|Sequence
    (:then_0
      (bind _actiontable (Variables|Default|GetActionTable)
        (:then
          (bind _outrownames (DataTable|GetDataTableRowNames _actiontable))
          (for _array_element _outrownames
            (bind _returnvalue (Utilities|GetDataTableRow (Variables|Default|GetActionTable) _array_element)
              (:then
                (Utilities|Array|Add (Variables|Default|GetActionDatas) _returnvalue)))))
        (:else)))
    (:then_1
      (bind _ascharacter (Utilities|Casting|CastToCharacter (Components|GetOwner)))
      (Variables|Default|SetOwnerCharacter _ascharacter))))

(fn ConstructionScript)

(fn BeginEquip)

(fn EndEquip
  (Variables|Default|SetEquipped true))

(fn Unequip
  (Variables|Default|SetEquipped false))

(fn GetEquipped
  (return (Variables|Default|GetEquipped)))

(fn AttachtoOwnerCharacter
  (params (InSocketName :type Name))
  (Transformation|AttachComponentToComponent (Variables|/Script/Engine.Character|GetMesh (Variables|Default|GetOwnerCharacter)) InSocketName "KeepRelative" "KeepRelative" "KeepRelative" true))

(fn IsExistAction
  (for _array_element (Variables|Default|GetActionDatas)
    (if (Utilities|Enum|Equal(Enum) (.type _array_element) (Variables|Default|GetWeaponType))
      (return true)))
  (return false))

(fn GetActions
  (for _array_element (Variables|Default|GetActionDatas)
    (if (and (Utilities|Enum|Equal(Enum) (.Type (Utilities|Struct|BreakFAction _array_element)) (Variables|Default|GetWeaponType)) (not (.Skill (Utilities|Struct|BreakFAction _array_element))))
      (Utilities|Array|Add (LocalVariables|GetActions) _array_element)))
  (return (LocalVariables|GetActions)))

(fn GetDamage
  (params (Index :type Integer) (Skill :type Boolean))
  (return (.damage (Utilities|Array|Get(acopy) (select Skill (Action|GetSkills) (Action|GetActions)) Index))))

(fn GetCameraShake
  (params (Index :type Integer) (Skill :type Boolean))
  (return (.camerashakeclass (Utilities|Array|Get(acopy) (select Skill (Action|GetSkills) (Action|GetActions)) Index))))

(fn GetCanMove
  (params (Index :type Integer) (Skill :type Boolean))
  (return (.canmove (Utilities|Array|Get(acopy) (select Skill (Action|GetSkills) (Action|GetActions)) Index))))

(fn GetEffect
  (params (Index :type Integer) (Skill :type Boolean))
  (bind _outactions (Action|GetActions))
  (bind _outskills (Action|GetSkills))
  (bind _returnvalue (select Skill _outskills _outactions))
  (bind _output (Utilities|Array|Get(acopy) _returnvalue Index))
  (return (.effect _output) (.effectlocation _output) (.effectscale _output) (.effectrotation _output)))

(fn GetSound
  (params (Index :type Integer) (Skill :type Boolean))
  (return (.soundcue (Utilities|Array|Get(acopy) (select Skill (Action|GetSkills) (Action|GetActions)) Index))))

(fn GetStop
  (params (Index :type Integer) (Skill :type Boolean))
  (return (.stop (Utilities|Array|Get(acopy) (select Skill (Action|GetSkills) (Action|GetActions)) Index))))

(fn PlayAction
  (params (Index :type Integer) (Skill :type Boolean))
  (bind _outactions (Action|GetActions))
  (bind _outskills (Action|GetSkills))
  (bind _ownercharacter (Variables|Default|GetOwnerCharacter))
  (bind _returnvalue (select Skill _outskills _outactions))
  (bind _output (Utilities|Array|Get(acopy) _returnvalue Index))
  (Animation|PlayAnimMontage (Variables|Default|GetOwnerCharacter) (.montage _output) (.playratio _output) "None")
  (if (Utilities|DoesObjectImplementInterface _ownercharacter "/Game/Interfaces/IWeapon.IWeapon_C")
    (if (Action|GetCanMove Index false)
      (Class|IWeapon|SetWeaponMove(Message) _ownercharacter)
      (else
        (Class|IWeapon|SetWeaponStop(Message) _ownercharacter)))))

(fn SendDamage
  (params (OtherActor :type Actor%20Object%20Reference) (Damage :type Float%20%28single-precision%29))
  (if (and (!= OtherActor (Variables|Default|GetOwnerCharacter)) (!= self OtherActor))
    (Game|Damage|ApplyDamage OtherActor Damage (Game|GetPlayerController 0) self)))

(fn DoAction)

(fn BeginAction)

(fn EndAction)

(fn GetSkills
  (for _array_element (Variables|Default|GetActionDatas)
    (if (and (Utilities|Enum|Equal(Enum) (.Type (Utilities|Struct|BreakFAction _array_element)) (Variables|Default|GetWeaponType)) (.Skill (Utilities|Struct|BreakFAction _array_element)))
      (Utilities|Array|Add (LocalVariables|GetSkills) _array_element)))
  (return (LocalVariables|GetSkills)))

(fn DoSubAction
  (params (KeyIndex :type Integer)))

(fn BeginSubAction)

(fn EndSubAction)