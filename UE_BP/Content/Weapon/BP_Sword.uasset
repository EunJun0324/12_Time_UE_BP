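; Sword weapon that moves between holster and hand sockets and drives its owner's combo attacks and two skills through state interfaces.
; Combo-window flags queue the next attack, while skills either lunge with an enlarged hit capsule (Launcher) or spawn a slash actor.
; Attacks spawn a ghost trail.
; Capsule overlaps apply indexed damage, camera shake, sound and hit-stop through global time dilation with a timer scaled to match.
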(fn ConstructionScript
  (|CallParentFunction))

(fn OnCollision
  (Collision|SetCollisionEnabled (Variables|Default|GetCapsule) "QueryAndPhysics"))

(fn OffCollsion
  (Collision|SetCollisionEnabled (Variables|Default|GetCapsule) "NoCollision"))

(fn RestoreStopTimer
  (Utilities|Time|SetGlobalTimeDilation 1.0))

(event Custom|Lock_EnableCombo
  ;[1 1 1] Combo
  (Variables|Default|SetEnable false))

(event Custom|UnLock_EnableCombo
  ;[1 1 1] Combo
  (Variables|Default|SetEnable true))

(event EventDoAction
  (bind _ownercharacter (Variables|Default|GetOwnerCharacter))
  ;[1 1 1] DoAction
  (|CallParentFunction)
  (if (CallFunction|IsExistAction)
    (if (Variables|Default|GetEnable)
      (Variables|Default|SetEnable false)
      (Variables|Default|SetExist true)
      (elif (Utilities|DoesObjectImplementInterface _ownercharacter "/Game/Interfaces/IState.IState_C")
        (bind _result (Class|IState|IsStateIdle(Message) _ownercharacter))
        (if _result
          (Class|IState|SetStateAction(Message) _ownercharacter)
          (CallFunction|PlayAction 0 false)
          (CallFunction|SpawnGhostTrail))))))

(event EventBeginAction
  ;[1 1 1] BeginAction
  (|CallParentFunction)
  (if (Variables|Default|GetExist)
    (Variables|Default|SetExist false)
    (Animation|StopAnimMontage (Variables|Default|GetOwnerCharacter) 0)
    (Math|Integer|IncrementInt (Variables|Default|GetIndex)
      (:%20%20
        (CallFunction|PlayAction (Variables|Default|GetIndex) false)))))

(event EventEndAction
  (bind _ownercharacter (Variables|Default|GetOwnerCharacter))
  (bind _ownercharacter_2 (Variables|Default|GetOwnerCharacter))
  ;[1 1 1] EndAction
  (|CallParentFunction)
  (Variables|Default|SetIndex 0)
  (Animation|StopAnimMontage _ownercharacter_2 0)
  (if (Utilities|DoesObjectImplementInterface _ownercharacter_2 "/Game/Interfaces/IState.IState_C")
    (Class|IState|SetStateIdle(Message) _ownercharacter)
    (if (Utilities|DoesObjectImplementInterface _ownercharacter "/Game/Interfaces/IWeapon.IWeapon_C")
      (Class|IWeapon|SetWeaponMove(Message) (Variables|Default|GetOwnerCharacter))
      (CallFunction|DestoryGhostTrail))))

(event Custom|SpawnGhostTrail
  (bind _ownercharacter (Variables|Default|GetOwnerCharacter))
  (bind _returnvalue (Transformation|GetActorLocation _ownercharacter))
  ;[1 1 1] GhostTrail
  (bind _returnvalue_2 (Game|SpawnActorfromClass "/Game/Weapon/BP_GhostTrail.BP_GhostTrail_C" (Math|Transform|MakeTransform (Math|Vector|MakeVector (.x _returnvalue) (.y _returnvalue) (- (.z _returnvalue) 9e+01))) "AlwaysSpawn" (Variables|Default|GetOwnerCharacter) 0))
  (Variables|Default|SetGhostTrail _returnvalue_2))

(event Custom|DestoryGhostTrail
  ;[1 1 1] GhostTrail
  (Actor|DestroyActor (Variables|Default|GetGhostTrail)))

(event EventBeginPlay
  ;[1 1 1] BeginPlay
  (|CallParentFunction)
  (CallFunction|AttachtoOwnerCharacter "Holster_Sword")
  (CallFunction|OffCollsion))

(event EventBeginEquip
  ;[1 1 1] Equip
  (|CallParentFunction)
  (CallFunction|AttachtoOwnerCharacter "Hand_Sword"))

(event EventEndEquip
  ;[1 1 1] Equip
  (|CallParentFunction)
  (CallFunction|AttachtoOwnerCharacter "Holster_Sword"))

(event OnComponentBeginOverlap(Capsule)
  (params (OverlappedComponent :type Primitive%20Component%20Object%20Reference) (OtherActor :type Actor%20Object%20Reference) (OtherComp :type Primitive%20Component%20Object%20Reference) (OtherBodyIndex :type Integer) (bFromSweep :type Boolean) (SweepResult :type Hit%20Result%20Structure%20%28by%20ref%29))
  ;[1 1 1] BeginOverlap
  (if (and (!= OtherActor (Variables|Default|GetOwnerCharacter)) (!= OtherActor self))
    (Utilities|FlowControl|Sequence
      (:then_0
        (|Damage OtherActor))
      (:then_1
        (|CameraShake))
      (:then_2
        (|Sound))
      (:then_3
        (Audio|Components|Audio|Stop)))))

(event Custom|Begin_Launcher
  (bind _capsule (Variables|Default|GetCapsule))
  (bind _ownercharacter (Variables|Default|GetOwnerCharacter))
  ;[1 1 1] BeginLauncher
  (Components|Capsule|SetCapsuleHalfHeight _capsule 84.0 true)
  (Components|Capsule|SetCapsuleRadius _capsule 84.0 true)
  (Physics|AddImpulse (Variables|/Script/Engine.Character|GetCharacterMovement _ownercharacter) (* (Transformation|GetActorForwardVector _ownercharacter) 5e+04) true))

(event Custom|Begin_Slash
  (bind _ownercharacter (Variables|Default|GetOwnerCharacter))
  ;[1 1 1] Begin_Slash
  (Game|SpawnActorfromClass "/Game/Weapon/BP_Slash.BP_Slash_C" (Math|Transform|MakeTransform (+ (Transformation|GetActorLocation _ownercharacter) "0.000000, 0,-90.000000") (Transformation|GetActorRotation _ownercharacter) "3.000000,1.500000,3.000000") "AlwaysSpawn" (Variables|Default|GetOwnerCharacter) 0))

(event EventDoSubAction
  (params (KeyIndex :type Integer))
  (bind _ownercharacter (Variables|Default|GetOwnerCharacter))
  ;[1 1 1] DoSubAction
  (|CallParentFunction KeyIndex)
  (if (Utilities|DoesObjectImplementInterface _ownercharacter "/Game/Interfaces/IState.IState_C")
    (bind _result (Class|IState|IsStateIdle(Message) _ownercharacter))
    (bind _result_2 (Math|Integer|DecrementInt KeyIndex)
      (:%20%20
        (Variables|Default|SetKey _result_2)
        (if _result
          (Class|IState|SetStateAction(Message) _ownercharacter)
          (CallFunction|PlayAction (Variables|Default|GetKey) true)
          (Variables|Default|SetIsSkill true)
          (CallFunction|SpawnGhostTrail))))))

(event EventBeginSubAction
  ;[1 1 1] BeginSubAction
  (|CallParentFunction)
  (switch int (Variables|Default|GetKey)
    (:0
      (CallFunction|BeginLauncher))
    (:1
      (CallFunction|BeginSlash))))

(event EventEndSubAction
  (bind _capsule (Variables|Default|GetCapsule))
  (bind _ownercharacter (Variables|Default|GetOwnerCharacter))
  ;[1 1 1] EndSubAction
  (|CallParentFunction)
  (Class|IState|SetStateIdle(Message) _ownercharacter)
  (Class|IWeapon|SetWeaponMove(Message) _ownercharacter)
  (CallFunction|DestoryGhostTrail)
  (Variables|Default|SetIsSkill false)
  (switch int (Variables|Default|GetKey)
    (:0
      (Components|Capsule|SetCapsuleHalfHeight _capsule 36.0 true)
      (Components|Capsule|SetCapsuleRadius _capsule 6.0 true))))