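; Shotgun weapon child Blueprint that moves between hand and holster sockets, with a separate launcher mesh for its skill.
; Primary and sub actions start only from the owner's idle state, and their end events restore it.
; The shot shoves the owner backward and line-traces forward, dealing distance-scaled damage to characters or leaving decals on other surfaces.
; The skill has an explosion event that spawns BP_Explosion ahead of the owner with camera shake.
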(fn ConstructionScript
  (|CallParentFunction))

(event EventBeginPlay
  ;[1 1 1] BeingPlay
  (|CallParentFunction)
  (CallFunction|AttachtoOwnerCharacter "Hand_Shotgun")
  (Utilities|Array|Add (Variables|Default|GetIgnoreActors) (Variables|Default|GetOwnerCharacter))
  (Transformation|AttachComponentToComponent (Variables|Default|GetLauncher) (Variables|/Script/Engine.Character|GetMesh (Variables|Default|GetOwnerCharacter)) "Holster_Launcher" "KeepRelative" "KeepRelative" "KeepRelative" true))

(event EventEndEquip
  ;[1 1 1] Equip
  (|CallParentFunction)
  (CallFunction|AttachtoOwnerCharacter "Holster_Shotgun"))

(event EventBeginEquip
  ;[1 1 1] Equip
  (|CallParentFunction)
  (CallFunction|AttachtoOwnerCharacter "Hand_Shotgun"))

(event EventDoAction
  (bind _ownercharacter (Variables|Default|GetOwnerCharacter))
  ;[1 1 1] DoAction
  (|CallParentFunction)
  (if (Utilities|DoesObjectImplementInterface _ownercharacter "/Game/Interfaces/IState.IState_C")
    (bind _result (Class|IState|IsStateIdle(Message) _ownercharacter))
    (if _result
      (Class|IState|SetStateAction(Message) _ownercharacter)
      (CallFunction|PlayAction 0 false))))

(event EventBeginAction
  (bind _ownercharacter (Variables|Default|GetOwnerCharacter))
  ;[1 1 1] BeginAction
  (|CallParentFunction)
  (Physics|AddImpulse (Variables|/Script/Engine.Character|GetCharacterMovement _ownercharacter) (* (Transformation|GetActorForwardVector _ownercharacter) -1e+03) true)
  (bind _outhit (Collision|LineTraceByChannel (Transformation|GetSocketLocation (Variables|Default|GetShotGun) "LineTrace") (+ (Transformation|GetSocketLocation (Variables|Default|GetShotGun) "LineTrace") (* (Transformation|GetActorForwardVector (Variables|Default|GetOwnerCharacter)) 1e+03)) "TraceTypeQuery1" false (Variables|Default|GetIgnoreActors) "ForDuration"))
  (if (.bBlockingHit (Collision|BreakHitResult _outhit))
    (if (!= (Variables|Default|GetOwnerCharacter) (.HitActor (Collision|BreakHitResult _outhit)))
      (Utilities|Casting|CastToCharacter (.HitActor (Collision|BreakHitResult _outhit))
        (:then
          (if (== (.Distance (Collision|BreakHitResult _outhit)) 0.0)
            (CallFunction|SendDamage (.HitActor (Collision|BreakHitResult _outhit)) (CallFunction|GetDamage 0 false))
            (else
              (CallFunction|SendDamage (.HitActor (Collision|BreakHitResult _outhit)) (* (CallFunction|GetDamage 0 false) (- 1.0 (/ (.Distance (Collision|BreakHitResult _outhit)) 1e+03)))))))
        (:CastFailed
          (Rendering|Decal|SpawnDecalatLocation "/Game/Materials/M_Decal_Inst.M_Decal_Inst" "5.000000,5.000000,5.000000" (.Location (Collision|BreakHitResult _outhit)) (Math|Conversions|RotationFromXVector (.ImpactNormal (Collision|BreakHitResult _outhit))) 0.0))))))

(event EventEndAction
  (bind _ownercharacter (Variables|Default|GetOwnerCharacter))
  (bind _ownercharacter_2 (Variables|Default|GetOwnerCharacter))
  ;[1 1 1] EndAction
  (|CallParentFunction)
  (Animation|StopAnimMontage _ownercharacter_2 0)
  (if (Utilities|DoesObjectImplementInterface _ownercharacter_2 "/Game/Interfaces/IState.IState_C")
    (Class|IState|SetStateIdle(Message) _ownercharacter)
    (if (Utilities|DoesObjectImplementInterface _ownercharacter "/Game/Interfaces/IWeapon.IWeapon_C")
      (Class|IWeapon|SetWeaponMove(Message) (Variables|Default|GetOwnerCharacter)))))

(event Custom|UnEquip_Launcher
  ;[1 1 1] Equip Launchar
  (Transformation|AttachComponentToComponent (Variables|Default|GetLauncher) (Variables|/Script/Engine.Character|GetMesh (Variables|Default|GetOwnerCharacter)) "Holster_Launcher" "KeepRelative" "KeepRelative" "KeepRelative" true))

(event Custom|Equip_Launcher
  ;[1 1 1] Equip Launchar
  (Transformation|AttachComponentToComponent (Variables|Default|GetLauncher) (Variables|/Script/Engine.Character|GetMesh (Variables|Default|GetOwnerCharacter)) "Hand_Launcher" "KeepRelative" "KeepRelative" "KeepRelative" true))

(event Custom|Begin_Explosion
  (bind _ownercharacter (Variables|Default|GetOwnerCharacter))
  ;[1 1 1] Begin_Explosion
  (Game|SpawnActorfromClass "/Game/Weapon/BP_Explosion.BP_Explosion_C" (Math|Transform|MakeTransform (+ (* (Transformation|GetActorForwardVector _ownercharacter) 6.5e+02) (Transformation|GetActorLocation _ownercharacter) "0.000000,0.000000,90.000000") (Transformation|GetActorRotation _ownercharacter) "2.000000,2.000000,2.000000") "AlwaysSpawn" (Variables|Default|GetOwnerCharacter) 0)
  (CameraShakes|StartCameraShake (Game|GetPlayerCameraManager 0) (CallFunction|GetCameraShake 0 true) 1.0 "CameraLocal" "0, 0, 0"))

(event EventEndSubAction
  (bind _ownercharacter (Variables|Default|GetOwnerCharacter))
  ;[1 1 1] EndSubAction
  (|CallParentFunction)
  (Class|IState|SetStateIdle(Message) _ownercharacter)
  (Class|IWeapon|SetWeaponMove(Message) _ownercharacter)
  (Variables|Default|SetIsSkill false)
  (switch int (Variables|Default|GetKey)))

(event EventBeginSubAction
  ;[1 1 1] BeginSubAction
  (|CallParentFunction)
  (CallFunction|BeginExplosion))

(event EventDoSubAction
  (params (KeyIndex :type Integer))
  (bind _ownercharacter (Variables|Default|GetOwnerCharacter))
  ;[1 1 1] DoSubAction
  (|CallParentFunction KeyIndex)
  (if (Utilities|DoesObjectImplementInterface _ownercharacter "/Game/Interfaces/IState.IState_C")
    (bind _result (Class|IState|IsStateIdle(Message) _ownercharacter))
    (bind _result_2 (Math|Integer|DecrementInt (Variables|Default|GetKey))
      (:%20%20
        (Variables|Default|SetKey _result_2)
        (if _result
          (Class|IState|SetStateAction(Message) _ownercharacter)
          (CallFunction|PlayAction 0 true)
          (Variables|Default|SetIsSkill true))))))