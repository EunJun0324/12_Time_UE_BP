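; Player character that fights with a sword and a shotgun, spawned at BeginPlay with the shotgun active.
; Action and skill inputs forward to the current weapon; switching, allowed only when idle, plays a data-table-driven equip montage and sets the Equip state.
; An enum state and movement flags gate actions.
; Dash turns toward velocity, then rolls or launches by impulse depending on weapon type, alongside walk, zoom and free-look camera controls.
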(event Input|ActionEvents|InputActionAction
  (params (Key :type Key%20Structure))
  ;[1 1 1] Action
  (:Pressed
    (Default|DoAction (Variables|Weapon|GetWeapon))))

(event Input|ActionEvents|InputActionSkill
  (params (Key :type Key%20Structure))
  ;[1 1 1] SubAction
  (:Pressed
    (Default|DoSubAction (Variables|Weapon|GetWeapon) (Math|Conversions|ToInteger(Byte) (Utilities|String|ToString(Text) (Class|KismetInputLibrary|KeyGetDisplayName Key))))))

(fn ConstructionScript
  (bind _springarm (Variables|Default|GetSpringArm))
  (Class|SkinnedMeshComponent|SetSkeletalMesh (Variables|Character|GetMesh) "/Game/Character/Mesh/SK_Mannequin.SK_Mannequin" true)
  (Transformation|SetRelativeLocationAndRotation (Variables|Character|GetMesh) "0,0.000000,-90.000000" "0,-70.000000, 0" false false)
  (Transformation|SetRelativeLocationAndRotation (Variables|Default|GetSpringArm) "0, 0,140.000000" "0,90.000000, 0" false false)
  (Utilities|FlowControl|Sequence
    (:then_0
      (Variables|/Script/Engine.SpringArmComponent|SetbUsePawnControlRotation _springarm true)
      (Transformation|SetRelativeLocation (Variables|Default|GetCamera) "-16.000000, 0,33.000000" false false)
      (Variables|Movement|SetCanMove true)
      (Variables|Zoom|SetZoomSpeed 1e+03)
      (Variables|Zoom|SetZoomRange "(X=100.000000,Y=500.000000)")
      (Variables|Default|SetbUseControllerRotationYaw true)
      (Variables|/Script/Engine.CharacterMovementComponent|SetbOrientRotationToMovement (Variables|Character|GetCharacterMovement) false))
    (:then_1
      (Variables|/Script/Engine.SpringArmComponent|SetbDoCollisionTest _springarm false))
    (:then_2
      (Variables|/Script/Engine.SpringArmComponent|SetTargetArmLength _springarm 1e+02))))

(event Custom|EndDash
  ;[1 1 1] Dash
  (Variables|Default|SetbUseControllerRotationYaw true)
  (Variables|/Script/Engine.CharacterMovementComponent|SetbOrientRotationToMovement (Variables|Character|GetCharacterMovement) false)
  (Utilities|FlowControl|Delay 3.0)
  (Variables|이동|SetCanDash true))

(event Input|ActionEvents|InputActionDash
  (params (Key :type Key%20Structure))
  (bind _returnvalue (Transformation|GetActorLocation))
  ;[1 1 1] Dash
  (:Pressed
    (bind _result (CallFunction|IsStateEquip))
    (if (Math|Boolean|ANDBoolean (not _result) (Variables|Movement|GetCanMove) (Variables|이동|GetCanDash))
      (Variables|Default|SetbUseControllerRotationYaw false)
      (Variables|/Script/Engine.CharacterMovementComponent|SetbOrientRotationToMovement (Variables|Character|GetCharacterMovement) true)
      (Variables|이동|SetCanDash false)
      (Transformation|SetActorRotation (Math|Rotator|FindLookatRotation _returnvalue (+ _returnvalue (Class|KismetMathLibrary|VectorNormal2D (Transformation|GetVelocity) 0.0001))))
      (bind _result_2 (CallFunction|IsSwitching))
      (if _result_2
        (Animation|PlayAnimMontage "/Game/Character/Montages/Roll_Montage.Roll_Montage" 1.5 "None")
        (else
          (Physics|AddImpulse (Variables|Character|GetCharacterMovement) (* (Transformation|GetActorForwardVector) 1.5e+04) true)
          (CallFunction|EndDash))))))

(event Input|ActionEvents|InputActionWalk
  (params (Key :type Key%20Structure))
  (bind _charactermovement (Variables|Character|GetCharacterMovement))
  ;[1 1 1] Walk
  (:Pressed
    (Variables|/Script/Engine.CharacterMovementComponent|SetMaxWalkSpeed _charactermovement 4e+02))
  (:Released
    (Variables|/Script/Engine.CharacterMovementComponent|SetMaxWalkSpeed _charactermovement 6e+02)))

(event Input|AxisEvents|InputAxisMoveForwad
  (params (AxisValue :type Float%20%28single-precision%29))
  ;[1 1 1] Move
  (if (Variables|Movement|GetCanMove)
    (Pawn|Input|AddMovementInput (Transformation|GetActorForwardVector) AxisValue false)))

(event Input|AxisEvents|InputAxisMoveRight
  (params (AxisValue :type Float%20%28single-precision%29))
  ;[1 1 1] Move
  (if (Variables|Movement|GetCanMove)
    (Pawn|Input|AddMovementInput (Transformation|GetActorRightVector) AxisValue false)))

(event Input|ActionEvents|InputActionFreeSight
  (params (Key :type Key%20Structure :default "None"))
  ;[1 1 1] FreeSight
  (:Pressed
    (Variables|Default|SetbUseControllerRotationYaw false))
  (:Released
    (Variables|Default|SetbUseControllerRotationYaw true)))

(event Input|AxisEvents|InputAxisVerticalLook
  (params (AxisValue :type Float%20%28single-precision%29))
  ;[1 1 1] Rotation
  (if (not (Variables|/Game/Weapon/BP_Sword.BP_Sword_C|GetIsSkill (Variables|Weapon|GetSword)))
    (Pawn|Input|AddControllerPitchInput AxisValue)))

(event Input|AxisEvents|InputAxisHorizontalLook
  (params (AxisValue :type Float%20%28single-precision%29))
  ;[1 1 1] Rotation
  (if (not (Variables|/Game/Weapon/BP_Sword.BP_Sword_C|GetIsSkill (Variables|Weapon|GetSword)))
    (Pawn|Input|AddControllerYawInput AxisValue)))

(event Input|AxisEvents|InputAxisZoom
  (params (AxisValue :type Float%20%28single-precision%29))
  (bind _zoomrange (Variables|Zoom|GetZoomRange))
  ;[1 1 1] Zoom
  (Variables|/Script/Engine.SpringArmComponent|SetTargetArmLength (Variables|Default|GetSpringArm) (Math|Float|Clamp(Float) (+ (* AxisValue (Variables|Zoom|GetZoomSpeed) (Utilities|Time|GetWorldDeltaSeconds)) (Variables|/Script/Engine.SpringArmComponent|GetTargetArmLength (Variables|Default|GetSpringArm))) (.x _zoomrange) (.y _zoomrange))))

(event EventBeginPlay
  (Utilities|FlowControl|Sequence
    (:then_0
      (|InitializeColor))
    (:then_1
      (|SpawnWeapons))
    (:then_2
      (|ReadDatas))))

(event Input|ActionEvents|InputActionSwitcing
  (params (Key :type Key%20Structure))
  ;[1 1 1] Switcing
  (:Pressed
    (bind _result (CallFunction|IsStateIdle))
    (if _result
      (bind _result_2 (CallFunction|IsSwitching))
      (if _result_2
        (CallFunction|WeaponChange (Variables|Weapon|GetShotgun))
        (else
          (CallFunction|WeaponChange (Variables|Weapon|GetSword)))))))

(fn GetWeaponCurrent
  (return (Variables|Weapon|GetWeapon)))

(fn IsStateAction
  (return (Utilities|Enum|Equal(Enum) (Variables|State|GetStateType) "NewEnumerator1")))

(fn IsStateDash
  (return (Utilities|Enum|Equal(Enum) (Variables|State|GetStateType) "NewEnumerator5")))

(fn IsStateDead
  (return (Utilities|Enum|Equal(Enum) (Variables|State|GetStateType) "NewEnumerator2")))

(fn IsStateEquip
  (return (Utilities|Enum|Equal(Enum) (Variables|State|GetStateType) "NewEnumerator4")))

(fn IsStateHitted
  (return (Utilities|Enum|Equal(Enum) (Variables|State|GetStateType) "NewEnumerator3")))

(fn IsStateIdle
  (return (Utilities|Enum|Equal(Enum) (Variables|State|GetStateType) "NewEnumerator0")))

(fn IsSwitching
  (bind _weapon (Variables|Weapon|GetWeapon)
    (:then
      (return (Utilities|Enum|Equal(Enum) (Variables|/Game/Weapon/BP_Weapon.BP_Weapon_C|GetWeaponType _weapon) "NewEnumerator0")))
    (:else)))

(fn SetStateAction
  (Variables|State|SetStateType "NewEnumerator1")
  (return false))

(fn SetStateDash
  (Variables|State|SetStateType "NewEnumerator5")
  (return false))

(fn SetStateDead
  (Variables|State|SetStateType "NewEnumerator2")
  (return false))

(fn SetStateEquip
  (Variables|State|SetStateType "NewEnumerator4")
  (return false))

(fn SetStateHitted
  (Variables|State|SetStateType "NewEnumerator3")
  (return false))

(fn SetStateIdle
  (Variables|State|SetStateType "NewEnumerator0")
  (return false))

(fn SetWeaponMove
  (Variables|Movement|SetCanMove true)
  (return false))

(fn SetWeaponStop
  (Variables|Movement|SetCanMove false)
  (return false))

(fn WeaponBeginEquip
  (bind _weapon (Variables|Weapon|GetWeapon)
    (:then
      (Default|BeginEquip _weapon)
      (CallFunction|SetStateIdle)
      (return false))
    (:else)))

(fn WeaponChange
  (params (InWeapon :type BP%20Weapon%20Object%20Reference))
  (bind _inweapon (LocalVariables|GetInWeapon)
    (:then
      (bind _output_get (Variables|Weapon|SetWeapon _inweapon))
      (CallFunction|PlayEquipMontage self (Variables|/Game/Weapon/BP_Weapon.BP_Weapon_C|GetWeaponType _output_get) (Variables|DataTable|GetEquipDatas))
      (CallFunction|SetStateEquip)
      (return true))
    (:else)))

(fn WeaponEndEquip
  (bind _result (CallFunction|IsSwitching))
  (if _result
    (Default|EndEquip (Variables|Weapon|GetShotgun))
    (else
      (Default|EndEquip (Variables|Weapon|GetSword))))
  (return false))